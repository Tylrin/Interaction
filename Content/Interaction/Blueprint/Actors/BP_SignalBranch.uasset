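; BP_SignalBranch is a signal-routing actor that acts as a conditional branch between interactable targets.
; On the authority, True and False commands set its stored condition; any other command sends each configured message to its target from the TrueSignal or FalseSignal list, chosen by that condition.
; The construction script shows a flip-flop icon when the first entry in each list targets itself to invert the condition, otherwise a branch icon.
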(event `/Interaction/InteractionSystem/Blueprint/BPI_InteractableActor.InteractionFromEvent`
  (params (Instigator :type "Actor Object Reference") (Command :type Name))
  ;[0 0 0] Event On Name Signal
  (`/Engine/EditorBlueprintResources/ActorMacros.Switch Has Authority`
    (:`Authority`
      (switch `name` Command
        (:`Default`
          (if (`self.ConditionValue`)
            (for _array_element (`self.TrueSignal`)
              (bind (_target _message) (break `/Interaction/InteractionSystem/Blueprint/Data/SInteractionCommand` _array_element))
              (message `/Interaction/InteractionSystem/Blueprint/BPI_InteractableActor.InteractionFromEvent` _target _target _message))
            (else
              (for _array_element_2 (`self.FalseSignal`)
                (bind (_target_2 _message_2) (break `/Interaction/InteractionSystem/Blueprint/Data/SInteractionCommand` _array_element_2))
                (message `/Interaction/InteractionSystem/Blueprint/BPI_InteractableActor.InteractionFromEvent` _target_2 _target_2 _message_2)))))
        (:`true`
          (set `self.ConditionValue` true))
        (:`false`
          (set `self.ConditionValue` false))))))

(fn `UserConstructionScript`
  (bind _icon (`self.Icon`))
  (bind (_target _message) (break `/Interaction/InteractionSystem/Blueprint/Data/SInteractionCommand` (`|GetArrayItem` (`self.TrueSignal`))))
  (bind (_target_2 _message_2) (break `/Interaction/InteractionSystem/Blueprint/Data/SInteractionCommand` (`|GetArrayItem` (`self.FalseSignal`))))
  ;[0 0 0] Construction Script
  (`parent.UserConstructionScript`)
  (if (and (== _target self) (== _message "false") (== _target_2 self) (== _message_2 "true"))
    (`BillboardComponent.SetSprite` _icon "/Interaction/InteractionSystem/Textures/T_Flipflop_Icon.T_Flipflop_Icon")
    (else
      (`BillboardComponent.SetSprite` _icon "/Interaction/InteractionSystem/Textures/T_Branch_Icon.T_Branch_Icon"))))