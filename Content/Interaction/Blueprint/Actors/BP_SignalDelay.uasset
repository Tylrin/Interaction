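; BP_SignalDelay is an interaction actor that relays incoming signals to its target after an adjustable delay.
; On the server, each command is queued with a parallel release timestamp, and new commands are dropped when an optional queue cap is reached.
; A looping timer scans for the first due entry, forwards its message and removes it, releasing at most one signal per tick.
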(event `self.ReceiveBeginPlay`
  ;[0.1529 0.7529 0.2099] Event Begin Play
  (`/Engine/EditorBlueprintResources/ActorMacros.Switch Has Authority`
    (:`Authority`
      (`KismetSystemLibrary.K2_SetTimer` null "DelayTimer" (`self.DelayTimerUpdateInterval`) true))))

(event `/Interaction/InteractionSystem/Blueprint/BPI_InteractableActor.InteractionFromEvent`
  (params (Instigator :type "Actor Object Reference") (Command :type Name))
  ;[0 0 0] Event On Name Signal
  (`/Engine/EditorBlueprintResources/ActorMacros.Switch Has Authority`
    (:`Authority`
      (if (`self.HasMaxQueueLenght`)
        (if (< (`KismetArrayLibrary.Array_Length` (`self.InteractionSignalTimeQueue`)) (`self.MaxQueueLength`))
          (`KismetArrayLibrary.Array_Add` (`self.InteractionSignalQueue`) (make `/Interaction/InteractionSystem/Blueprint/Data/SInteractionCommand` Instigator Command) :!label _label)
          (`KismetArrayLibrary.Array_Add` (`self.InteractionSignalTimeQueue`) (+ (`KismetSystemLibrary.GetGameTimeInSeconds`) (`self.Delay`))))
        (else
          (goto _label))))))

(fn `DelayTimer`
  ;[0 0 0] Delay Timer
  (bind (_returnvalue _index) (`self.GetCurrentDelaySignalIndex`))
  (if _returnvalue
    (message `/Interaction/InteractionSystem/Blueprint/BPI_InteractableActor.InteractionFromEvent` (`self.Target`) null (`.Message_3_1458EE714DB746860C09BB8630342FDA` (break `/Interaction/InteractionSystem/Blueprint/Data/SInteractionCommand` (`|GetArrayItem` (`self.InteractionSignalQueue`) _index))))
    (`KismetArrayLibrary.Array_Remove` (`self.InteractionSignalQueue`) _index)
    (`KismetArrayLibrary.Array_Remove` (`self.InteractionSignalTimeQueue`) _index)
    (return)
    (else
      (return))))

(fn `GetCurrentDelaySignalIndex`
  (returns (ReturnValue :type Boolean) (Index :type Integer))
  (locals (LocalIndex :type Integer) (LocalInteractionSignalTime :type "Float (double-precision)") (LocalReturnValue :type Boolean))
  ;[0 0 0] Get Current Delay Signal Index
  (for _index (range (+ (`KismetArrayLibrary.Array_LastIndex` (`self.InteractionSignalQueue`)) 1))
    (bind _output (`|GetArrayItem` (`self.InteractionSignalTimeQueue`) _index))
    (if (<= _output (`KismetSystemLibrary.GetGameTimeInSeconds`))
      (set `local.LocalInteractionSignalTime` _output)
      (set `local.LocalIndex` _index)
      (set `local.LocalReturnValue` true)
      (break)))
  (if (`local.LocalReturnValue`)
    (return true (`local.LocalIndex`))
    (else
      (return false 0))))

(fn `GetDelay`
  (returns (Delay :type "Float (double-precision)"))
  (return (`self.Delay`)))

(fn `SetDelay`
  (params (Delay :type "Float (double-precision)"))
  (set `self.Delay` Delay))

(fn `UserConstructionScript`
  (`parent.UserConstructionScript`))