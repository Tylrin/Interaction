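; Signal logic gate actor that combines boolean inputs from registered instigators using AND, OR or XOR (exactly one true).
; On authority, True/False commands update the sender's entry in an input map, then re-evaluate and send the Activation or Deactivation signal messages to their targets.
; Or/And/Xor commands switch gate type at runtime without re-evaluating; the construction script sets the matching icon.
; Inverted gates are intended via swapping the two signal lists.
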(event `/Interaction/InteractionSystem/Blueprint/BPI_InteractableActor.InteractionFromEvent`
  (params (Instigator :type "Actor Object Reference") (Command :type Name))
  (bind _inputactivationtargets (`self.InputActivationTargets`))
  ;[0 0 0] Event On Name Signal
  (`/Engine/EditorBlueprintResources/ActorMacros.Switch Has Authority`
    (:`Authority`
      (switch `name` Command
        (:`or`
          (`self.SetGateType` "NewEnumerator1") ; NAND / NOR / XNOR Should be posible by switching the Activation Signal and Deactivation Signal
        )
        (:`and`
          (`self.SetGateType` "NewEnumerator0"))
        (:`xor`
          (`self.SetGateType` "NewEnumerator3"))
        (:`true`
          (bind _returnvalue (`self.HasActivationTarget` Instigator))
          (if _returnvalue
            (`BlueprintMapLibrary.Map_Add` _inputactivationtargets Instigator true)
            (bind _returnvalue_2 (`self.CheckGate` :!label _label))
            (if _returnvalue_2
              (for _array_element (`self.ActivationSignal`)
                (bind (_target _message) (break `/Interaction/InteractionSystem/Blueprint/Data/SInteractionCommand` _array_element))
                (message `/Interaction/InteractionSystem/Blueprint/BPI_InteractableActor.InteractionFromEvent` _target null _message))
              (else
                (for _array_element_2 (`self.DeactivationSignal`)
                  (bind (_target_2 _message_2) (break `/Interaction/InteractionSystem/Blueprint/Data/SInteractionCommand` _array_element_2))
                  (message `/Interaction/InteractionSystem/Blueprint/BPI_InteractableActor.InteractionFromEvent` _target_2 null _message_2))))))
        (:`false`
          (bind _returnvalue_3 (`self.HasActivationTarget` Instigator))
          (if _returnvalue_3
            (`BlueprintMapLibrary.Map_Add` _inputactivationtargets Instigator)
            (goto _label)))))))

(fn `CheckAND`
  (returns (ReturnValue :type Boolean))
  (locals (LocalReturnValue :type Boolean :default true))
  ;[0.9734 0.1356 0.1356] Check AND
  (bind _values (`BlueprintMapLibrary.Map_Values` (`self.InputActivationTargets`)))
  (for _array_element _values
    (if (not _array_element)
      (set `local.LocalReturnValue` false)
      (break)))
  (return (`local.LocalReturnValue`)))

(fn `CheckGate`
  (returns (ReturnValue :type Boolean))
  ;[0.9734 0.1356 0.1356] Check Gate
  (switch `/Interaction/InteractionSystem/Blueprint/Data/ELogicGateType` (`self.GateType`)
    (:`NewEnumerator0`
      (bind _returnvalue (`self.CheckAND`))
      (return _returnvalue))
    (:`NewEnumerator1`
      (bind _returnvalue_2 (`self.CheckOR`))
      (return _returnvalue_2))
    (:`NewEnumerator3`
      (bind _returnvalue_3 (`self.CheckXOR`))
      (return _returnvalue_3))))

(fn `CheckOR`
  (returns (ReturnValue :type Boolean))
  (locals (LocalReturnValue :type Boolean))
  ;[0.9734 0.1356 0.1356] Check OR
  (bind _values (`BlueprintMapLibrary.Map_Values` (`self.InputActivationTargets`)))
  (for _array_element _values
    (if _array_element
      (set `local.LocalReturnValue` true)
      (break)))
  (return (`local.LocalReturnValue`)))

(fn `CheckXOR`
  (returns (ReturnValue :type Boolean))
  (locals (LocalReturnValue :type Boolean))
  ;[0.9734 0.1356 0.1356] Check XOR
  (bind _values (`BlueprintMapLibrary.Map_Values` (`self.InputActivationTargets`)))
  (for _array_element _values
    (if _array_element
      (if (`local.LocalReturnValue`)
        (set `local.LocalReturnValue` false)
        (break)
        (else
          (set `local.LocalReturnValue` true)))))
  (return (`local.LocalReturnValue`)))

(fn `HasActivationTarget`
  (params (Key :type "Actor Object Reference (by ref)"))
  (returns (ReturnValue :type Boolean))
  (return (`.ReturnValue` (`BlueprintMapLibrary.Map_Find` (`self.InputActivationTargets`) Key))))

(fn `SetGateType`
  (params (GateType :type "/Interaction/InteractionSystem/Blueprint/Data/ELogicGateType Enum" :default "NewEnumerator0"))
  ;[0.9734 0.1356 0.1356] Set Gate Type
  (set `self.GateType` GateType))

(fn `UserConstructionScript`
  (bind _icon (`self.Icon`))
  ;[0.1529 0.7529 0.2099] Construction Script
  (`parent.UserConstructionScript`)
  (switch `/Interaction/InteractionSystem/Blueprint/Data/ELogicGateType` (`self.GateType`)
    (:`NewEnumerator0`
      (`BillboardComponent.SetSprite` _icon "/Interaction/InteractionSystem/Textures/T_And_Icon.T_And_Icon"))
    (:`NewEnumerator1`
      (`BillboardComponent.SetSprite` _icon "/Interaction/InteractionSystem/Textures/T_Or_Icon.T_Or_Icon"))
    (:`NewEnumerator3`
      (`BillboardComponent.SetSprite` _icon "/Interaction/InteractionSystem/Textures/T_Xor_Icon.T_Xor_Icon"))))