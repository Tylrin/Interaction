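; BP_SignalTi is an interaction actor that acts as a timer, relaying messages to a list of target objects.
; On the authority, it can auto-start a looping timer at BeginPlay, and incoming interaction commands start, pause, unpause or toggle it.
; The timer is set by function name, and TimerTransmitSignal sends each target its configured message through the same interaction event, so signal actors can be chained.
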(event `self.ReceiveBeginPlay`
  ;[0.1529 0.7529 0.2099] Event Begin Play
  (`/Engine/EditorBlueprintResources/ActorMacros.Switch Has Authority`
    (:`Authority`
      (if (`self.AutoStart`)
        (`KismetSystemLibrary.K2_SetTimer` null (`self.TimerName`) (`self.TimerInterval`) true)))))

(event `InteractionFromEvent_1`
  (params (Command :type Name))
  ;[0 0 0] Event On Name Signal
  (`/Engine/EditorBlueprintResources/ActorMacros.Switch Has Authority`
    (:`Authority`
      (switch `name` Command
        (:`start`
          ;;[1 1 1 0.25] Timer
          (`KismetSystemLibrary.K2_SetTimer` null (`self.TimerName`) (`self.TimerInterval`) true))
        (:`pause`
          (`KismetSystemLibrary.K2_PauseTimer` null (`self.TimerName`)))
        (:`unpause`
          (`KismetSystemLibrary.K2_UnPauseTimer` null (`self.TimerName`)))
        (:`toggle`
          (if (`KismetSystemLibrary.K2_IsTimerPaused` null (`self.TimerName`))
            (`KismetSystemLibrary.K2_UnPauseTimer` null (`self.TimerName`))
            (else
              (`KismetSystemLibrary.K2_PauseTimer` null (`self.TimerName`)))))))))

(fn `TimerTransmitSignal`
  ;[0 0 0] Timer Transmit Signal
  (for _array_element _
    (bind (_target _message) (break `` _array_element))
    (message `/Game/Interaction/Blueprint/Actors/BP_SignalTi.InteractionFromEvent` _target null _message)))

(fn `UserConstructionScript`)