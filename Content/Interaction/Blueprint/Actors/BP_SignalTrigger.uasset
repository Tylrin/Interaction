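; Trigger volume actor that sends interaction messages to configured targets when allowed actors enter or leave it.
; The construction script adds a box, sphere or capsule collision component from the selected shape and size settings.
; On authority only, overlaps matching an exact class list are tracked and fire the activation signals on every entry.
; Deactivation signals fire on each exit, or only when the last tracked actor leaves if that option is set.
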(event `Event_ComponentBeginOverlap`
  (params (Actor :type "Actor Object Reference"))
  ;[0 0 0] Event OnComponentBeginOverlap
  (`/Engine/EditorBlueprintResources/ActorMacros.Switch Has Authority`
    (:`Authority`
      (if (`self.IsOverlapObject` Actor)
        (`KismetArrayLibrary.Array_AddUnique` (`self.ObjectsOverlaping`) Actor)
        (for _array_element (`self.ActivationSignal`)
          (bind (_target _message) (break `/Interaction/InteractionSystem/Blueprint/Data/SInteractionCommand` _array_element))
          (message `/Interaction/InteractionSystem/Blueprint/BPI_InteractableActor.InteractionFromEvent` _target Actor _message))))))

(event `Event_ComponentEndOverlap`
  (params (Actor :type "Actor Object Reference"))
  (bind _objectsoverlaping (`self.ObjectsOverlaping`))
  ;[0 0 0] Event OnComponentEndOverlap
  (`/Engine/EditorBlueprintResources/ActorMacros.Switch Has Authority`
    (:`Authority`
      (if (`self.IsOverlapObject` Actor)
        (`KismetArrayLibrary.Array_RemoveItem` _objectsoverlaping Actor)
        (if (`self.DedeactivateOnLastLeave`)
          (if (<= (`KismetArrayLibrary.Array_Length` _objectsoverlaping) 0)
            (for _array_element (`self.DeactivationSignal`) :!label _label
              (bind (_target _message) (break `/Interaction/InteractionSystem/Blueprint/Data/SInteractionCommand` _array_element))
              (message `/Interaction/InteractionSystem/Blueprint/BPI_InteractableActor.InteractionFromEvent` _target Actor _message)))
          (else
            (goto _label)))))))

(event `self.BoxCollision.OnComponentBeginOverlap`
  (params (OverlappedComponent :type "PrimitiveComponent Object Reference") (OtherActor :type "Actor Object Reference") (OtherComp :type "PrimitiveComponent Object Reference") (OtherBodyIndex :type Integer) (bFromSweep :type Boolean) (SweepResult :type "HitResult Structure (by ref)"))
  ;[0 0 0] On Component Begin Overlap
  (`self.Event_ComponentBeginOverlap` OtherActor))

(event `self.BoxCollision.OnComponentEndOverlap`
  (params (OverlappedComponent :type "PrimitiveComponent Object Reference") (OtherActor :type "Actor Object Reference") (OtherComp :type "PrimitiveComponent Object Reference") (OtherBodyIndex :type Integer))
  ;[0 0 0] On Component End Overlap
  (`self.Event_ComponentEndOverlap` OtherActor))

(event `self.SphereCollision.OnComponentBeginOverlap`
  (params (OverlappedComponent :type "PrimitiveComponent Object Reference") (OtherActor :type "Actor Object Reference") (OtherComp :type "PrimitiveComponent Object Reference") (OtherBodyIndex :type Integer) (bFromSweep :type Boolean) (SweepResult :type "HitResult Structure (by ref)"))
  ;[0 0 0] On Component Begin Overlap
  (`self.Event_ComponentBeginOverlap` OtherActor))

(event `self.SphereCollision.OnComponentEndOverlap`
  (params (OverlappedComponent :type "PrimitiveComponent Object Reference") (OtherActor :type "Actor Object Reference") (OtherComp :type "PrimitiveComponent Object Reference") (OtherBodyIndex :type Integer))
  ;[0 0 0] On Component End Overlap
  (`self.Event_ComponentEndOverlap` OtherActor))

(event `self.CapsuleCollision.OnComponentBeginOverlap`
  (params (OverlappedComponent :type "PrimitiveComponent Object Reference") (OtherActor :type "Actor Object Reference") (OtherComp :type "PrimitiveComponent Object Reference") (OtherBodyIndex :type Integer) (bFromSweep :type Boolean) (SweepResult :type "HitResult Structure (by ref)"))
  ;[0 0 0] On Component Begin Overlap
  (`self.Event_ComponentBeginOverlap` OtherActor))

(event `self.CapsuleCollision.OnComponentEndOverlap`
  (params (OverlappedComponent :type "PrimitiveComponent Object Reference") (OtherActor :type "Actor Object Reference") (OtherComp :type "PrimitiveComponent Object Reference") (OtherBodyIndex :type Integer))
  ;[0 0 0] On Component End Overlap
  (`self.Event_ComponentEndOverlap` OtherActor))

(fn `IsOverlapObject`
  (params (Actor :type "Actor Object Reference"))
  (returns (ReturnValue :type Boolean))
  (locals (LocalReturn :type Boolean))
  ;[0.3916 1 0.3372] Is Overlap Object
  (for _array_element (`self.OverlapObjects`)
    (if (== _array_element (`GameplayStatics.GetObjectClass` Actor))
      (set `local.LocalReturn` true)
      (break)))
  (return (`local.LocalReturn`)))

(fn `UserConstructionScript`
  (`parent.UserConstructionScript`)
  (switch `|SwitchEnum` (`self.GeometryShape`)
    (:`NewEnumerator0`
      (bind _returnvalue (`AddComponent|NODE_AddBoxComponent-0`))
      (bind _output_get (set `self.BoxCollision` _returnvalue))
      (`BoxComponent.SetBoxExtent` _output_get (`self.BoxExtent`) true)
      (`SceneComponent.SetHiddenInGame` (`self.BoxCollision`) (`self.HiddeInGame`) false))
    (:`NewEnumerator1`
      (bind _returnvalue_2 (`AddComponent|NODE_AddSphereComponent-0`))
      (bind _output_get_2 (set `self.SphereCollision` _returnvalue_2))
      (`SphereComponent.SetSphereRadius` _output_get_2 (`self.SphereRadius`) true)
      (`SceneComponent.SetHiddenInGame` (`self.SphereCollision`) (`self.HiddeInGame`) false))
    (:`NewEnumerator2`
      (bind _returnvalue_3 (`AddComponent|NODE_AddCapsuleComponent-0`))
      (bind _output_get_3 (set `self.CapsuleCollision` _returnvalue_3))
      (`CapsuleComponent.SetCapsuleSize` _output_get_3 (`self.CapsuleRadius`) (`self.CapsuleHalfHeight`) true)
      (`SceneComponent.SetHiddenInGame` (`self.CapsuleCollision`) (`self.HiddeInGame`) false))))