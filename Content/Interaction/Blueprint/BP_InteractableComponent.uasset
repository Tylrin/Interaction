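; Actor component, by its name, that marks something as interactable and tracks which actors are currently viewing it.
; Focus and unfocus calls add or remove the actor in a duplicate-free ViewingActors list, which HasViewingActor checks for any viewer.
; It also holds a gameplay tag container with add and remove helpers.
; UpdateInteractable is an empty stub, and the Component argument of the focus calls is unused.
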(fn `AddInteractableTag`
  (params (Tag :type "GameplayTag Structure"))
  (`BlueprintGameplayTagLibrary.AddGameplayTag` (`self.InteractableTags`) Tag))

(fn `AddViewingActor`
  (params (Actor :type "Actor Object Reference"))
  (`KismetArrayLibrary.Array_AddUnique` (`self.ViewingActors`) Actor))

(fn `FocusInteractable`
  (params (Actor :type "Actor Object Reference") (Component :type "PrimitiveComponent Object Reference"))
  (`self.AddViewingActor` Actor))

(fn `HasViewingActor`
  (returns (HasViewingActor :type Boolean))
  (return (> (`KismetArrayLibrary.Array_Length` (`self.ViewingActors`)) 0)))

(fn `RemoveInteractableTag`
  (params (Tag :type "GameplayTag Structure"))
  (returns (HasRemovedTag :type Boolean))
  (bind _returnvalue (`BlueprintGameplayTagLibrary.RemoveGameplayTag` (`self.InteractableTags`) Tag))
  (return _returnvalue))

(fn `RemoveViewingActor`
  (params (Actor :type "Actor Object Reference (by ref)"))
  (`KismetArrayLibrary.Array_RemoveItem` (`self.ViewingActors`) Actor))

(fn `UnfocusInteractable`
  (params (Actor :type "Actor Object Reference") (Component :type "PrimitiveComponent Object Reference"))
  (`self.RemoveViewingActor` Actor))

(fn `UpdateInteractable`
  (params (Actor :type "Actor Object Reference") (Component :type "PrimitiveComponent Object Reference")))