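; BP_SignalActorSpawner is an interaction-driven actor that spawns a configurable actor class at a random point inside a box.
; An authority-only interaction event triggers Spawn, which keeps the spawner's rotation and randomizes scale within set limits.
; UniformScale applies the X range to every axis but still rolls each separately, so scale can be non-uniform.
; The construction script sizes the box and sets its in-game visibility.
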(event `/Interaction/InteractionSystem/Blueprint/BPI_InteractableActor.InteractionFromEvent`
  (params (Instigator :type "Actor Object Reference") (Command :type Name))
  ;[0 0 0] Interface // Actor Interaction
  (`/Engine/EditorBlueprintResources/ActorMacros.Switch Has Authority`
    (:`Authority`
      (switch `name` Command
        (:`Spawn`
          (`self.Event Spawn`))))))

(event `Event Spawn`
  (bind _returnvalue (`KismetMathLibrary.RandomFloatInRange` (.x (`self.SpawnScaleMin`)) (.x (`self.SpawnScaleMax`))))
  ;[0 0 0] Spawn
  (`|SpawnActorFromClass` (`self.ActorToSpawn`) (`KismetMathLibrary.MakeTransform` (`KismetMathLibrary.RandomPointInBoundingBox` (.location (`self.GetTransform`)) (`self.SpawnBoxSize`)) (.rotation (`self.GetTransform`)) (`KismetMathLibrary.SelectVector` (`KismetMathLibrary.MakeVector` _returnvalue _returnvalue _returnvalue) (`KismetMathLibrary.MakeVector` (`KismetMathLibrary.RandomFloatInRange` (.x (`self.SpawnScaleMin`)) (.x (`self.SpawnScaleMax`))) (`KismetMathLibrary.RandomFloatInRange` (.y (`self.SpawnScaleMin`)) (.y (`self.SpawnScaleMax`))) (`KismetMathLibrary.RandomFloatInRange` (.z (`self.SpawnScaleMin`)) (.z (`self.SpawnScaleMax`)))) (`self.UniformScale`))) "Undefined" "OverrideRootScale" null null))

(fn `UserConstructionScript`
  (`parent.UserConstructionScript`)
  (`SceneComponent.SetHiddenInGame` (`self.Box`) (`self.HiddeInGame`) false)
  (`BoxComponent.SetBoxExtent` (`self.Box`) (`self.SpawnBoxSize`) false))