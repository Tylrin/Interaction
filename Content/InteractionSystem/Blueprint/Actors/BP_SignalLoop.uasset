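; BP_SignalLoop is an interaction-system actor that relays an incoming interaction event as repeated signals to other targets.
; On authority only, it loops by the Loop count, sending each InteractionSignalLoop entry's message to its target through InteractionFromEventMessage.
; After the loop finishes, it sends the InteractionSignalCompleted messages once to their targets.
; All repeats run back to back with no delay between them.
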(event `/Interaction/InteractionSystem/Blueprint/BPI_InteractableActor.InteractionFromEvent`
  (params (Instigator :type "Actor Object Reference") (Command :type Name))
  ;[0 0 0] On Name Signal
  (`/Engine/EditorBlueprintResources/ActorMacros.Switch Has Authority`
    (:`Authority`
      (for _ (range (+ (`self.Loop`) 1))
        (for _array_element (`self.InteractionSignalLoop`)
          (bind (_target _message) (break `/Interaction/InteractionSystem/Blueprint/Data/SInteractionCommand` _array_element))
          (message `/Interaction/InteractionSystem/Blueprint/BPI_InteractableActor.InteractionFromEvent` _target null _message)))
      (for _array_element_2 (`self.InteractionSignalCompleted`)
        (bind (_target_2 _message_2) (break `/Interaction/InteractionSystem/Blueprint/Data/SInteractionCommand` _array_element_2))
        (message `/Interaction/InteractionSystem/Blueprint/BPI_InteractableActor.InteractionFromEvent` _target_2 null _message_2)))))

(fn `UserConstructionScript`
  (`parent.UserConstructionScript`))